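; Behavior tree task that picks a random search point for an AI around the last seen location.
; On execute, it gets a random navigable point within the search-mode radius of that blackboard location and writes it to the point location key.
; It then increments the searching index key, counting search attempts, and always finishes successfully without checking whether a point was found.
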(event `self.ReceiveExecuteAI`
  (params (OwnerController :type "AIController Object Reference") (ControlledPawn :type "Pawn Object Reference"))
  (`BTFunctionLibrary.SetBlackboardValueAsVector` (`self.PointLocationKeySelector`) (`NavigationSystemV1.K2_GetRandomLocationInNavigableRadius` (`BTFunctionLibrary.GetBlackboardValueAsVector` (`self.LastSeenLocationKeySelector`)) (`self.RadiusInSearchMode`) null null))
  (`BTFunctionLibrary.SetBlackboardValueAsInt` (`self.SearchingIndexKeySelector`) (+ (`BTFunctionLibrary.GetBlackboardValueAsInt` (`self.SearchingIndexKeySelector`)) 1))
  (`self.FinishExecute` true))