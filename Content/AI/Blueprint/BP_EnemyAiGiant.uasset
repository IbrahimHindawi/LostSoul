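; Giant enemy AI character that changes movement speed with its controller's alert state and plays stomp and search animations.
; BeginPlay caches the default walk speed and derives a follow speed from a multiplier.
; Tick polls the alert state on BP_AiController and applies walk speed when patrolling or follow speed when following.
; MeleeAttack and SearchAnim events only play their montages, with no damage or detection logic here.
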(event `self.ReceiveBeginPlay`
  (bind _output_get (set `self.WalkSpeed` (`CharacterMovementComponent.MaxWalkSpeed` (`self.CharacterMovement`))))
  (set `self.FollowSpeed` (* _output_get (`self.FollowSpeedMultiplier`))))

(event `self.ReceiveTick`
  (params (DeltaSeconds :type "Float (single-precision)"))
  (bind _asbp_ai_controller (cast `/Game/AI/Blueprint/BP_AiController` (`AIBlueprintHelperLibrary.GetAIController` self)))
  (switch `/Game/AI/Blueprint/AlertState` (`/Game/AI/Blueprint/BP_AiController.AlertState` _asbp_ai_controller)
    (:`NewEnumerator0`
      (set `CharacterMovementComponent.MaxWalkSpeed` (`self.WalkSpeed`) (`self.CharacterMovement`)))
    (:`NewEnumerator1`
      (set `CharacterMovementComponent.MaxWalkSpeed` (`self.FollowSpeed`) (`self.CharacterMovement`)))))

(event `/Game/AI/Blueprint/EnemyMeleeInterface.MeleeAttack`
  (`|PlayMontage` (`self.Mesh`) "/Game/Giant/anim/StompMon.StompMon" 0.9))

(event `/Game/AI/Blueprint/EnemyMeleeInterface.SearchAnim`
  (`|PlayMontage` (`self.Mesh`) "/Game/Giant/anim/SearchingAnimMon.SearchingAnimMon"))

(fn `UserConstructionScript`)